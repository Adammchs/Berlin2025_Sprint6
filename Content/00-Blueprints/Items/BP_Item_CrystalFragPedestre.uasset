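; Puzzle pedestal that accepts a crystal fragment item and checks whether it holds the correct combination of crystal types.
; On sphere overlap it snaps the crystal into place, forces the player to ungrab, and compares its fragment list to five hardcoded types in any order.
; A match turns the light green and signals the enigma as valid; otherwise it turns red.
; Removing the crystal frees the pedestal and resets either material or light color.
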(event OnComponentBeginOverlap(Sphere)
  (params (OverlappedComponent :type Primitive%20Component%20Object%20Reference) (OtherActor :type Actor%20Object%20Reference) (OtherComp :type Primitive%20Component%20Object%20Reference) (OtherBodyIndex :type Integer) (bFromSweep :type Boolean) (SweepResult :type Hit%20Result%20Structure%20%28by%20ref%29))
  (Utilities|IsValid (Variables|Default|GetCrystalOnPiedestral)
    (:Is%20Not%20Valid
      (bind _asbp_item_crystals_frag (Utilities|Casting|CastToBP_Item_CrystalsFrag OtherActor))
      (bind _output_get (Variables|Default|SetCrystalOnPiedestral _asbp_item_crystals_frag))
      (Transformation|AttachComponentToComponent _output_get (Variables|Default|GetCrystalPos) "None" "SnapToTarget" "SnapToTarget" "KeepWorld" true)
      (Default|ForceUngrab (Variables|Default|GetPlayerRef))
      (Variables|Default|SetGood (Utilities|Array|MakeArray))
      (bind _fraglist (Default|GetFragList (Variables|Default|GetCrystalOnPiedestral)))
      (for _array_element _fraglist
        (Utilities|Array|Add (Variables|Default|GetGood) (Variables|/Game/00-Blueprints/Items/BP_Item_CrystalsFrag.BP_Item_CrystalsFrag_C|GetCrystalType _array_element)))
      (if (Math|Boolean|ANDBoolean (Utilities|Array|ContainsItem (Variables|Default|GetGood) "NewEnumerator0") (Utilities|Array|ContainsItem (Variables|Default|GetGood) "NewEnumerator1") (Utilities|Array|ContainsItem (Variables|Default|GetGood) "NewEnumerator2") (Utilities|Array|ContainsItem (Variables|Default|GetGood) "NewEnumerator3") (Utilities|Array|ContainsItem (Variables|Default|GetGood) "NewEnumerator6") (== (Utilities|Array|Length (Variables|Default|GetGood)) 5))
        (CallFunction|GoodCrystal)
        (Development|PrintString "GoodCrystal")
        (Default|CallEnigmaIsValid)
        (else
          (CallFunction|WrongCrystal)
          (Development|PrintString "WrongCrystal")))
      (Variables|Default|SetAlreadyHasACrystalOn true))))

(event OnComponentEndOverlap(Sphere)
  (params (OverlappedComponent :type Primitive%20Component%20Object%20Reference) (OtherActor :type Actor%20Object%20Reference) (OtherComp :type Primitive%20Component%20Object%20Reference) (OtherBodyIndex :type Integer))
  (bind _good (Variables|Default|GetGood))
  (if (== OtherActor (Variables|Default|GetCrystalOnPiedestral))
    (Utilities|Casting|CastToBP_Item_CrystalsFrag OtherActor)
    (if (Math|Boolean|ANDBoolean (Utilities|Array|ContainsItem _good "NewEnumerator0") (Utilities|Array|ContainsItem _good "NewEnumerator1") (Utilities|Array|ContainsItem _good "NewEnumerator2") (Utilities|Array|ContainsItem _good "NewEnumerator3") (Utilities|Array|ContainsItem _good "NewEnumerator6") (== (Utilities|Array|Length _good) 5))
      (Rendering|Material|SetMaterial (Variables|Default|GetSM_Activated) 0 "/Engine/BasicShapes/BasicShapeMaterial.BasicShapeMaterial")
      (else
        (Rendering|Components|Light|SetLightColor (Variables|Default|GetLightComponent0) "(R=1.000000,G=1.000000,B=1.000000,A=1.000000)" true)))
    (Variables|Default|SetAlreadyHasACrystalOn false)
    (Variables|Default|SetCrystalOnPiedestral 0)))

(event Custom|WrongCrystal
  (Rendering|Components|Light|SetLightColor (Variables|Default|GetLightComponent0) "(R=1.000000,G=0.102599,B=0.000000,A=1.000000)" true))

(event Custom|GoodCrystal
  (Rendering|Components|Light|SetLightColor (Variables|Default|GetLightComponent0) "(R=0.000000,G=1.000000,B=0.097419,A=1.000000)" true))

(event EventBeginPlay
  (bind _asbp_fpsplayer (Utilities|Casting|CastToBP_FPSPlayer (Game|GetPlayerCharacter 0)))
  (Variables|Default|SetPlayerRef _asbp_fpsplayer)
  (|CallParentFunction))

(fn ConstructionScript
  (|CallParentFunction))