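; BP_Item_CrystalFuser is a two-pedestal item that fuses crystal fragments.
; Each overlap sphere claims the first BP_Item_CrystalsFrag to enter, snaps it to its slot and forces the player to release their grab.
; When both slots are filled it calls Fuse on one fragment with the other, and end overlap frees a slot.
; CheckCrystalPos tests an ID for good or wrong crystal with debug prints, but is not called within this graph.
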(event OnComponentBeginOverlap(Sphere)
  (params (OverlappedComponent :type Primitive%20Component%20Object%20Reference) (OtherActor :type Actor%20Object%20Reference) (OtherComp :type Primitive%20Component%20Object%20Reference) (OtherBodyIndex :type Integer) (bFromSweep :type Boolean) (SweepResult :type Hit%20Result%20Structure%20%28by%20ref%29))
  (bind _crystalonpiedestral_0 (Variables|Default|GetCrystalOnPiedestral_0))
  (Utilities|IsValid (Variables|Default|GetCrystalOnPiedestral)
    (:Is%20Not%20Valid
      (bind _asbp_item_crystals_frag (Utilities|Casting|CastToBP_Item_CrystalsFrag OtherActor))
      (bind _output_get (Variables|Default|SetCrystalOnPiedestral _asbp_item_crystals_frag))
      (Transformation|AttachComponentToComponent _output_get (Variables|Default|GetCrystalPos) "None" "SnapToTarget" "SnapToTarget" "KeepWorld" true)
      (Default|ForceUngrab (Variables|Default|GetPlayerRef))
      (Utilities|IsValid (Variables|Default|GetCrystalOnPiedestral)
        (:Is%20Valid
          (Utilities|IsValid _crystalonpiedestral_0
            (:Is%20Valid
              (Default|Fuse (Variables|Default|GetCrystalOnPiedestral) _crystalonpiedestral_0))))))))

(event OnComponentEndOverlap(Sphere)
  (params (OverlappedComponent :type Primitive%20Component%20Object%20Reference) (OtherActor :type Actor%20Object%20Reference) (OtherComp :type Primitive%20Component%20Object%20Reference) (OtherBodyIndex :type Integer))
  (if (== OtherActor (Variables|Default|GetCrystalOnPiedestral))
    (Variables|Default|SetCrystalOnPiedestral 0)))

(event OnComponentBeginOverlap(Sphere1)
  (params (OverlappedComponent :type Primitive%20Component%20Object%20Reference) (OtherActor :type Actor%20Object%20Reference) (OtherComp :type Primitive%20Component%20Object%20Reference) (OtherBodyIndex :type Integer) (bFromSweep :type Boolean) (SweepResult :type Hit%20Result%20Structure%20%28by%20ref%29))
  (bind _crystalonpiedestral (Variables|Default|GetCrystalOnPiedestral))
  (Utilities|IsValid (Variables|Default|GetCrystalOnPiedestral_0)
    (:Is%20Not%20Valid
      (bind _asbp_item_crystals_frag (Utilities|Casting|CastToBP_Item_CrystalsFrag OtherActor))
      (bind _output_get (Variables|Default|SetCrystalOnPiedestral_0 _asbp_item_crystals_frag))
      (Transformation|AttachComponentToComponent _output_get (Variables|Default|GetCrystalPos1) "None" "SnapToTarget" "SnapToTarget" "KeepWorld" true)
      (Default|ForceUngrab (Variables|Default|GetPlayerRef))
      (Utilities|IsValid _crystalonpiedestral
        (:Is%20Valid
          (Utilities|IsValid (Variables|Default|GetCrystalOnPiedestral_0)
            (:Is%20Valid
              (Default|Fuse _crystalonpiedestral (Variables|Default|GetCrystalOnPiedestral_0)))))))))

(event OnComponentEndOverlap(Sphere1)
  (params (OverlappedComponent :type Primitive%20Component%20Object%20Reference) (OtherActor :type Actor%20Object%20Reference) (OtherComp :type Primitive%20Component%20Object%20Reference) (OtherBodyIndex :type Integer))
  (if (== OtherActor (Variables|Default|GetCrystalOnPiedestral_0))
    (Variables|Default|SetCrystalOnPiedestral_0 0)))

(event EventBeginPlay
  (bind _asbp_fpsplayer (Utilities|Casting|CastToBP_FPSPlayer (Game|GetPlayerCharacter 0)))
  (Variables|Default|SetPlayerRef _asbp_fpsplayer)
  (|CallParentFunction))

(fn ConstructionScript
  (|CallParentFunction))