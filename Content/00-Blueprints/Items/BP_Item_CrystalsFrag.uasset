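; Crystal fragment item whose emotion type (Anger, Sadness, Hope, etc.) sets its material, particles, looping-timeline motion, sound and light color.
; Fuse teleports another fragment onto this one, hides its mesh and particles, stores it, and blends material vector parameters through a count-weighted average.
; Unfuse re-shows and detaches stored fragments, then rebuilds this crystal's original type material, without clearing the stored list.
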(event Custom|Fuse
  (params (CrystalFrag :type BP%20Item%20Crystals%20Frag%20Object%20Reference))
  (Transformation|SetActorLocation CrystalFrag (Transformation|GetActorLocation) false true)
  (Rendering|SetVisibility (Variables|/Game/00-Blueprints/Items/BP_MasterItem.BP_MasterItem_C|GetSM_Shape CrystalFrag) false false)
  (Rendering|SetVisibility (Variables|BP_Item_CrystalsFrag_C|GetP_Crystal_1 CrystalFrag) false false)
  (Utilities|Array|Add (Variables|Default|GetCrystalFrags) CrystalFrag)
  (Utilities|FlowControl|Sequence
    (:then_0
      (CallFunction|SetColortoAverage CrystalFrag "Color_2"))
    (:then_1
      (CallFunction|SetColortoAverage CrystalFrag "Gradient_Color_1"))
    (:then_2
      (CallFunction|SetColortoAverage CrystalFrag "Gradient_Color_1.5"))
    (:then_3
      (CallFunction|SetColortoAverage CrystalFrag "Speed_1"))
    (:then_4
      (CallFunction|SetColortoAverage CrystalFrag "Tile_1"))
    (:then_5
      (CallFunction|SetColortoAverage CrystalFrag "Color_3"))
    (:then_6
      (CallFunction|SetColortoAverage CrystalFrag "Speed_2"))
    (:then_7
      (CallFunction|SetColortoAverage CrystalFrag "Tile_2"))
    (:then_8
      (CallFunction|SetColortoAverage CrystalFrag "Color_Fresnel"))
    (:then_9
      (CallFunction|SetColortoAverage CrystalFrag "Color_Fresnel_Inner"))))

(event Custom|Unfuse
  (for _array_element (Variables|Default|GetCrystalFrags)
    (Rendering|SetVisibility (Variables|/Game/00-Blueprints/Items/BP_MasterItem.BP_MasterItem_C|GetSM_Shape _array_element) true false)
    (Rendering|SetVisibility (Variables|BP_Item_CrystalsFrag_C|GetP_Crystal_1 _array_element) true false)
    (Transformation|DetachFromActor _array_element "KeepWorld" "KeepWorld" "KeepWorld"))
  (switch Utilities|FlowControl|Switch|SwitchonE_CrystalsType (Variables|Default|GetCrystalType)
    (:NewEnumerator0
      (bind _returnvalue (Rendering|Material|CreateDynamicMaterialInstance "/Game/Crystals/Material/M_Crystal_Inst3.M_Crystal_Inst3" "None" "None" :!class /Script/Engine.KismetMaterialLibrary))
      (Variables|Default|SetCrystalMaterial _returnvalue))
    (:NewEnumerator1
      (bind _returnvalue_2 (Rendering|Material|CreateDynamicMaterialInstance "/Game/Crystals/Material/M_Crystal_Inst4.M_Crystal_Inst4" "None" "None" :!class /Script/Engine.KismetMaterialLibrary))
      (Variables|Default|SetCrystalMaterial _returnvalue_2))
    (:NewEnumerator2
      (bind _returnvalue_3 (Rendering|Material|CreateDynamicMaterialInstance "/Game/Crystals/Material/M_Crystal_Inst6.M_Crystal_Inst6" "None" "None" :!class /Script/Engine.KismetMaterialLibrary))
      (Variables|Default|SetCrystalMaterial _returnvalue_3))
    (:NewEnumerator3
      (bind _returnvalue_4 (Rendering|Material|CreateDynamicMaterialInstance "/Game/Crystals/Material/M_Crystal_Inst9_2.M_Crystal_Inst9_2" "None" "None" :!class /Script/Engine.KismetMaterialLibrary))
      (Variables|Default|SetCrystalMaterial _returnvalue_4))
    (:NewEnumerator4
      (bind _returnvalue_5 (Rendering|Material|CreateDynamicMaterialInstance "/Game/Crystals/Material/M_Crystal_Inst1_2.M_Crystal_Inst1_2" "None" "None" :!class /Script/Engine.KismetMaterialLibrary))
      (Variables|Default|SetCrystalMaterial _returnvalue_5))
    (:NewEnumerator5
      (bind _returnvalue_6 (Rendering|Material|CreateDynamicMaterialInstance "/Game/Crystals/Material/M_Crystal_Inst10.M_Crystal_Inst10" "None" "None" :!class /Script/Engine.KismetMaterialLibrary))
      (Variables|Default|SetCrystalMaterial _returnvalue_6))
    (:NewEnumerator6
      (bind _returnvalue_7 (Rendering|Material|CreateDynamicMaterialInstance "/Game/Crystals/Material/M_Crystal_1.M_Crystal_1" "None" "None" :!class /Script/Engine.KismetMaterialLibrary))
      (Variables|Default|SetCrystalMaterial _returnvalue_7)))
  (Rendering|Material|SetMaterial (Variables|Default|GetSM_Shape) 0 (Variables|Default|GetCrystalMaterial)))

(event EventBeginPlay
  (bind _sm_shape (Variables|Default|GetSM_Shape))
  (|CallParentFunction)
  (switch Utilities|FlowControl|Switch|SwitchonE_CrystalsType (Variables|Default|GetCrystalType)
    (:NewEnumerator0
      (Variables|Default|SetCrystalSFX "/Game/02-Musics_SFX/Crystals/chert_Cue.chert_Cue")
      (Variables|Default|SetCrystalMesh "/Game/Crystals/Mesh/SM_Crystal_3.SM_Crystal_3")
      (bind _returnvalue (Rendering|Material|CreateDynamicMaterialInstance "/Game/Crystals/Material/M_Crystal_Inst3.M_Crystal_Inst3" "None" "None" :!class /Script/Engine.KismetMaterialLibrary))
      (Variables|Default|SetCrystalMaterial _returnvalue)
      (Variables|Default|SetCrystalVFX "/Game/Crystals/Particles/P_Crystal_3.P_Crystal_3")
      (Variables|Default|SetLightColor "(R=1.000000,G=0.145098,B=0.145098,A=1.000000)"))
    (:NewEnumerator1
      (Variables|Default|SetCrystalSFX "/Game/02-Musics_SFX/Crystals/esker_Cue.esker_Cue")
      (Variables|Default|SetCrystalMesh "/Game/Crystals/Mesh/SM_Crystal_3.SM_Crystal_3")
      (bind _returnvalue_2 (Rendering|Material|CreateDynamicMaterialInstance "/Game/Crystals/Material/M_Crystal_Inst4.M_Crystal_Inst4" "None" "None" :!class /Script/Engine.KismetMaterialLibrary))
      (Variables|Default|SetCrystalMaterial _returnvalue_2)
      (Variables|Default|SetCrystalVFX "/Game/Crystals/Particles/P_Crystal_5.P_Crystal_5")
      (Variables|Default|SetLightColor "(R=0.105882,G=0.454902,B=1.000000,A=1.000000)"))
    (:NewEnumerator2
      (Variables|Default|SetCrystalSFX "/Game/02-Musics_SFX/Crystals/feldspar_Cue.feldspar_Cue")
      (Variables|Default|SetCrystalMesh "/Game/Crystals/Mesh/SM_Crystal_3.SM_Crystal_3")
      (bind _returnvalue_3 (Rendering|Material|CreateDynamicMaterialInstance "/Game/Crystals/Material/M_Crystal_Inst6.M_Crystal_Inst6" "None" "None" :!class /Script/Engine.KismetMaterialLibrary))
      (Variables|Default|SetCrystalMaterial _returnvalue_3)
      (Variables|Default|SetCrystalVFX "/Game/Crystals/Particles/P_Crystal_7.P_Crystal_7")
      (Variables|Default|SetLightColor "(R=0.176471,G=1.000000,B=0.223529,A=1.000000)"))
    (:NewEnumerator3
      (Variables|Default|SetCrystalSFX "/Game/02-Musics_SFX/Crystals/riebeck_Cue.riebeck_Cue")
      (Variables|Default|SetCrystalMesh "/Game/Crystals/Mesh/SM_Crystal_3.SM_Crystal_3")
      (bind _returnvalue_4 (Rendering|Material|CreateDynamicMaterialInstance "/Game/Crystals/Material/M_Crystal_Inst9_2.M_Crystal_Inst9_2" "None" "None" :!class /Script/Engine.KismetMaterialLibrary))
      (Variables|Default|SetCrystalMaterial _returnvalue_4)
      (Variables|Default|SetCrystalVFX "/Game/Crystals/Particles/P_Crystal_9.P_Crystal_9")
      (Variables|Default|SetLightColor "(R=1.000000,G=0.905882,B=0.235294,A=1.000000)"))
    (:NewEnumerator4
      (Variables|Default|SetCrystalSFX "/Game/02-Musics_SFX/Crystals/SC_Fear.SC_Fear")
      (Variables|Default|SetCrystalMesh "/Game/Crystals/Mesh/SM_Crystal_3.SM_Crystal_3")
      (bind _returnvalue_5 (Rendering|Material|CreateDynamicMaterialInstance "/Game/Crystals/Material/M_Crystal_Inst1_2.M_Crystal_Inst1_2" "None" "None" :!class /Script/Engine.KismetMaterialLibrary))
      (Variables|Default|SetCrystalMaterial _returnvalue_5)
      (Variables|Default|SetCrystalVFX "/Game/Crystals/Particles/P_Crystal_1.P_Crystal_1")
      (Variables|Default|SetLightColor "(R=1.000000,G=0.266667,B=0.980392,A=1.000000)"))
    (:NewEnumerator5
      (Variables|Default|SetCrystalSFX "/Game/02-Musics_SFX/Crystals/SC_Remission.SC_Remission")
      (Variables|Default|SetCrystalMesh "/Game/Crystals/Mesh/SM_Crystal_3.SM_Crystal_3")
      (bind _returnvalue_6 (Rendering|Material|CreateDynamicMaterialInstance "/Game/Crystals/Material/M_Crystal_Inst10.M_Crystal_Inst10" "None" "None" :!class /Script/Engine.KismetMaterialLibrary))
      (Variables|Default|SetCrystalMaterial _returnvalue_6)
      (Variables|Default|SetCrystalVFX "/Game/Crystals/Particles/P_Crystal_10.P_Crystal_10")
      (Variables|Default|SetLightColor "(R=1.000000,G=0.356863,B=0.121569,A=1.000000)"))
    (:NewEnumerator6
      (Variables|Default|SetCrystalSFX "/Game/02-Musics_SFX/Crystals/solanum_Cue.solanum_Cue")
      (Variables|Default|SetCrystalMesh "/Game/Crystals/Mesh/SM_Crystal_3.SM_Crystal_3")
      (bind _returnvalue_7 (Rendering|Material|CreateDynamicMaterialInstance "/Game/Crystals/Material/M_Crystal_1.M_Crystal_1" "None" "None" :!class /Script/Engine.KismetMaterialLibrary))
      (Variables|Default|SetCrystalMaterial _returnvalue_7)
      (Variables|Default|SetCrystalVFX "/Game/Crystals/Particles/P_Crystal_10.P_Crystal_10")
      (Variables|Default|SetLightColor "(R=1.000000,G=1.000000,B=1.000000,A=1.000000)")))
  (Audio|Components|Audio|SetSound (Variables|Default|GetAudio) (Variables|Default|GetCrystalSFX))
  (Audio|Components|Audio|Play (Variables|Default|GetAudio) 0.0)
  (Components|StaticMesh|SetStaticMesh _sm_shape (Variables|Default|GetCrystalMesh))
  (Rendering|Material|SetMaterial _sm_shape 0 (Variables|Default|GetCrystalMaterial))
  (Effects|Components|ParticleSystem|SetTemplate (Variables|Default|GetP_Crystal_1) (Variables|Default|GetCrystalVFX))
  (Rendering|Components|Light|SetLightColor (Variables|Default|GetPointLight) (Variables|Default|GetLightColor) true)
  (bind _z (Timeline|Timeline Play)
    (:Update
      (Transformation|SetRelativeLocation (Variables|Default|GetSM_Shape) (Math|Vector|MakeVector 0.0 0.0 _z) false false))))

(fn ConstructionScript
  (|CallParentFunction))

(fn Average
  (params (Value1 :type Float%20%28double-precision%29) (Value2 :type Float%20%28double-precision%29) (Weight1 :type Integer) (Weight2 :type Integer))
  (return (/ (+ (* Value1 Weight1) (* Value2 Weight2)) (+ Weight1 Weight2))))

(fn SetColortoAverage
  (params (self2 :type BP%20Item%20Crystals%20Frag%20Object%20Reference) (Name :type Name))
  (bind _crystalmaterial (Variables|Default|GetCrystalMaterial))
  (bind _crystalfrags (Variables|Default|GetCrystalFrags))
  (bind _returnvalue (Utilities|Array|Length _crystalfrags))
  (bind _returnvalue_2 (+ _returnvalue 1))
  (bind _returnvalue_3 (Rendering|Material|GetVectorParameterValue (Variables|BP_Item_CrystalsFrag_C|GetCrystalMaterial self2) Name :!class /Script/Engine.MaterialInstanceDynamic))
  (bind _returnvalue_4 (Rendering|Material|GetVectorParameterValue _crystalmaterial Name :!class /Script/Engine.MaterialInstanceDynamic))
  (bind _result (CallFunction|Average (.r _returnvalue_3) (.r _returnvalue_4) 1 _returnvalue_2))
  (bind _result_2 (CallFunction|Average (.g _returnvalue_3) (.g _returnvalue_4) 1 _returnvalue_2))
  (bind _result_3 (CallFunction|Average (.b _returnvalue_3) (.b _returnvalue_4) 1 _returnvalue_2))
  (Rendering|Material|SetVectorParameterValue _crystalmaterial Name (Utilities|Struct|MakeLinearColor _result _result_2 _result_3 1.0) :!class /Script/Engine.MaterialInstanceDynamic))